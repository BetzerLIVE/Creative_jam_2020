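; BP_SHouse1 is a destructible house actor that players can punch to destroy for experience.
; On each punch, it subtracts the attacking character's punch damage from its remaining health through its Destructible component or interface.
; When health drops to zero or below, it adds its Exp value to that character's current experience and destroys itself.
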(event `self.Destructible.OnPunch`
  (params (Character :type "creativejamCharacter Object Reference"))
  (bind _destructible (`self.Destructible`))
  (bind _returnvalue (`DestructibleComponent.GetRemainingHealth` _destructible))
  (`DestructibleComponent.SetHealth` _destructible (- _returnvalue (`creativejamCharacter.PunchAttackDamage` Character)))
  (bind _returnvalue_2 (`DestructibleComponent.GetRemainingHealth` _destructible))
  (if (<= _returnvalue_2 0.0)
    (set `creativejamCharacter.CurrentExp` (+ (`creativejamCharacter.CurrentExp` Character) (`self.exp`)) Character)
    (`self.K2_DestroyActor`)))

(fn `UserConstructionScript`)