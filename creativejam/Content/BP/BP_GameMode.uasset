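; Game mode Blueprint that opens the game on a title screen and tracks whether the player has won.
; On BeginPlay it creates the UI_TitleScreen widget, adds it to the viewport and shows the mouse cursor.
; Every Tick it casts the player character to creativejamCharacter and sets its own Win flag only when that character is on level 10 with its Win flag set.
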(event `self.ReceiveBeginPlay`
  (bind _returnvalue (`GameplayStatics.GetPlayerController` 0))
  (bind _returnvalue_2 (`|GenericCreateObject` "/Game/UI/UI_TitleScreen.UI_TitleScreen_C" _returnvalue))
  (`UserWidget.AddToViewport` _returnvalue_2 0)
  (set `PlayerController.bShowMouseCursor` true _returnvalue))

(event `self.ReceiveTick`
  (params (DeltaSeconds :type "Float (single-precision)"))
  (bind _ascreativejam_character (cast `creativejamCharacter` (`GameplayStatics.GetPlayerCharacter` 0)))
  (set `self.Win` (and (== (`creativejamCharacter.Currentlevel` _ascreativejam_character) 10) (`creativejamCharacter.bWin` _ascreativejam_character))))

(fn `UserConstructionScript`)